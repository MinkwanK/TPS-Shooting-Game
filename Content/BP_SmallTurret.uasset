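; BP_SmallTurret is a small turret whose firing and death visuals follow its BCanFire and BDead flags.
; Every Tick, BCanFire activates both gun barrel components and spawns a gunshot sound each frame, otherwise deactivating the barrels.
; BDead swaps the intact mesh for the damaged one and activates a Niagara effect.
; The graph only reads these flags; BeginPlay just prints the object name.
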(event `self.ReceiveBeginPlay`
  (`KismetSystemLibrary.PrintString` (`KismetSystemLibrary.GetObjectName` self)))

(event `self.ReceiveTick`
  (params (DeltaSeconds :type "Float (single-precision)"))
  (bind __bdead (`self._bDead`))
  (bind _gun_barrel_l (`self.Gun_Barrel_L`))
  (if (`self._bCanFire`)
    (`ActorComponent.Activate` _gun_barrel_l true)
    (`ActorComponent.Activate` (`self.Gun_Barrel_R`) true)
    (`GameplayStatics.SpawnSoundAtLocation` "/Game/Gun+357+Magnum.Gun+357+Magnum" (`self.K2_GetActorLocation`) (struct) 1.0 1.0 0.0 null null)
    (else
      (`ActorComponent.Deactivate` _gun_barrel_l)
      (`ActorComponent.Deactivate` (`self.Gun_Barrel_R`))))
  (`SceneComponent.SetVisibility` (`self.Mesh`) (not (`self._bDead`)) true)
  (`SceneComponent.SetVisibility` (`self.DamagedMesh`) __bdead true)
  (`ActorComponent.SetActive` (`self.Niagara`) __bdead false))

(fn `UserConstructionScript`)