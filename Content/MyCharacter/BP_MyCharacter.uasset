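; Player character Blueprint that manages in-game UI, pause and game-over flow, and gun visuals.
; BeginPlay in the InGame level creates the HUD and caches the BP_GameStageTimer actor.
; Tick polls that timer and the death flag to show game over or, while unpaused, toggle the cursor by stage and drive the fire Niagara effect and reload magazine visibility.
; Tab opens the pause menu and pauses the game.
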(event `Game Pause Event`
  (bind _returnvalue (`GameplayStatics.GetPlayerController` 0))
  (bind _pause_menu_reference (`self.Pause Menu Reference`))
  ;[1 1 1] 게임 일시중지
  (`/Engine/EditorBlueprintResources/StandardMacros.IsValid` (`self.Pause Menu Reference`)
    (:`Is Valid`
      _)
    (:`Is Not Valid`
      (bind _returnvalue_2 (`|CreateWidget` "/Game/UI/BP_PauseMenu.BP_PauseMenu_C"))
      (set `self.Pause Menu Reference` _returnvalue_2)))
  (set `PlayerController.bShowMouseCursor` true _returnvalue)
  (`WidgetBlueprintLibrary.SetInputMode_UIOnlyEx` _returnvalue _pause_menu_reference)
  (`UserWidget.AddToViewport` _pause_menu_reference 0)
  (set `self._bPaused` true)
  (`GameplayStatics.SetGamePaused` true))

(event `Game State Event`
  (bind _returnvalue (`GameplayStatics.GetPlayerController` 0))
  ;[1 1 1] 게임 상태에 따른 UI 변환 및 게임 상태 변환 이벤트
  (`/Engine/EditorBlueprintResources/StandardMacros.IsValid` (`self.GameStageTimer Reference`)
    (:`Is Valid`
      (bind _asgame_stage_timer (cast `GameStageTimer` (`self.GameStageTimer Reference`)))
      (switch `EInGameState` (`GameStageTimer.InGameEnum` _asgame_stage_timer)
        (:`GameReadyState`
          (set `PlayerController.bShowMouseCursor` false _returnvalue :!label _label))
        (:`GameStartState`
          (goto _label))
        (:`GameRestState`
          (set `PlayerController.bShowMouseCursor` true _returnvalue))))))

(event `self.ReceiveBeginPlay`
  (bind _returnvalue (`GameplayStatics.GetCurrentLevelName` true))
  (if (`KismetStringLibrary.EqualEqual_StrStr` _returnvalue "InGame")
    (bind _returnvalue_2 (`|CreateWidget` "/Game/UI/BP_PlayerHUD.BP_PlayerHUD_C"))
    (bind _output_get (set `self.HUD Reference` _returnvalue_2))
    (`UserWidget.AddToViewport` _output_get 0)
    (`WidgetBlueprintLibrary.SetInputMode_GameOnly` (`GameplayStatics.GetPlayerController` 0))
    (bind _returnvalue_3 (`GameplayStatics.GetActorOfClass` "/Game/BP_GameStageTimer.BP_GameStageTimer_C"))
    (set `self.GameStageTimer Reference` _returnvalue_3)))

(event `Activate Gun Effect`
  ;[1 1 1] 총기 이펙트 이벤트
  (`ActorComponent.SetActive` (`self.Niagara`) (`self._bFire`) false)
  (`SceneComponent.SetHiddenInGame` (`self.Mag`) (not (`self._bReload`)) false))

(event `Game Over Event`
  (bind _returnvalue (`GameplayStatics.GetPlayerController` 0))
  ;[1 1 1] 게임오버이벤트
  (bind _returnvalue_2 (`|CreateWidget` "/Game/UI/BP_GameOver.BP_GameOver_C"))
  (set `PlayerController.bShowMouseCursor` true _returnvalue)
  (`WidgetBlueprintLibrary.SetInputMode_UIOnlyEx` _returnvalue (`/Game/UI/BP_GameOver.GameEndBtn` _returnvalue_2) "LockOnCapture")
  (`UserWidget.AddToViewport` _returnvalue_2 0)
  (`GameplayStatics.SetGamePaused` true))

(event `self.ReceiveTick`
  (params (DeltaSeconds :type "Float (single-precision)"))
  (if (or (`|EnumEquality` (`GameStageTimer.InGameEnum` (`self.GameStageTimer Reference`)) "GameEndState") (`self._bDead`))
    (`self.Game Over Event`)
    (elif (not (`self._bPaused`))
      (`self.Game State Event`)
      (`self.Activate Gun Effect`))))

(event `Key|Tab`
  (params (Key :type "Key Structure"))
  (:`Pressed`
    (set `self._bPaused` true)
    (`self.Game Pause Event`)))

(fn `Game Over Function`
  (`GameplayStatics.SetGamePaused` true))

(fn `UserConstructionScript`)